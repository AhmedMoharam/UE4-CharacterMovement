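; DarkSuperMan_BP is the DarkSuperMan character Blueprint, handling player camera and movement input.
; Axis inputs drive controller pitch and yaw, and movement follows the control rotation's yaw only.
; Holding Run switches the ExtendedMovementComponent from facing controller rotation to facing the movement direction, and releasing it switches back.
; BeginPlay caches the mesh's DarkSuperMan animation Blueprint instance.
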(event EventBeginPlay
  (bind _asdark_super_man_anim_bp (Utilities|Casting|CastToDarkSuperMan_Anim_BP (Components|SkeletalMesh|GetAnimInstance (Variables|Character|GetMesh))))
  (Variables|Reference|SetSuperMan_Anim_BP _asdark_super_man_anim_bp))

(event Collision|EventActorBeginOverlap
  (params (OtherActor :type Actor%20Object%20Reference)))

(event EventTick
  (params (DeltaSeconds :type Float%20%28single-precision%29)))

(event Input|ActionEvents|InputActionRun
  (params (Key :type Key%20Structure))
  (bind _extendedmovementcomponent (Variables|Default|GetExtendedMovementComponent))
  ;[1 1 1] Basic Movement
  (:Pressed
    (Variables|/Game/DarkSuperMan/BluePrints/ExtendedMovementComponent.ExtendedMovementComponent_C|SetOrient%20Rotation%20to%20Controller%20Rotation _extendedmovementcomponent false)
    (Variables|/Game/DarkSuperMan/BluePrints/ExtendedMovementComponent.ExtendedMovementComponent_C|SetOrient%20Rotation%20to%20Movement _extendedmovementcomponent true))
  (:Released
    (Variables|/Game/DarkSuperMan/BluePrints/ExtendedMovementComponent.ExtendedMovementComponent_C|SetOrient%20Rotation%20to%20Controller%20Rotation _extendedmovementcomponent true)
    (Variables|/Game/DarkSuperMan/BluePrints/ExtendedMovementComponent.ExtendedMovementComponent_C|SetOrient%20Rotation%20to%20Movement _extendedmovementcomponent false)))

(event Input|AxisEvents|InputAxisCameraUD
  (params (AxisValue :type Float%20%28single-precision%29))
  ;[1 1 1] Camera
  (Pawn|Input|AddControllerPitchInput AxisValue))

(event Input|AxisEvents|InputAxisCameraRL
  (params (AxisValue :type Float%20%28single-precision%29))
  ;[1 1 1] Camera
  (Pawn|Input|AddControllerYawInput AxisValue))

(event Input|AxisEvents|InputAxisForWard_Backward
  (params (AxisValue :type Float%20%28single-precision%29))
  ;[1 1 1] Basic Movement
  (Pawn|Input|AddMovementInput (Math|Vector|GetForwardVector (Math|Rotator|MakeRotator 0.0 0.0 (.yaw (Pawn|GetControlRotation :!class /Script/Engine.Pawn)))) AxisValue false))

(event Input|AxisEvents|InputAxisRight_Left
  (params (AxisValue :type Float%20%28single-precision%29))
  ;[1 1 1] Basic Movement
  (Pawn|Input|AddMovementInput (Math|Vector|GetRightVector (Math|Rotator|MakeRotator 0.0 0.0 (.yaw (Pawn|GetControlRotation :!class /Script/Engine.Pawn)))) AxisValue false))

(fn ConstructionScript)