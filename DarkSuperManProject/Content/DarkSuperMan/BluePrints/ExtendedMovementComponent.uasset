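; Actor component for the DarkSuperMan_BP character that turns it toward the controller's facing while it moves.
; BeginPlay casts the owner and caches it as the character reference.
; Each tick with non-zero velocity, it uses FixedTurn to step the actor's yaw toward control yaw at RotationYawRate, scaled by delta time.
; The new rotation is applied through the CharacterMovement component's MoveUpdatedComponent rather than by setting actor rotation.
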(event EventBeginPlay
  (bind _ascharacter (Utilities|Casting|CastToCharacter (Components|GetOwner)))
  (bind _asdark_super_man_bp (Utilities|Casting|CastToDarkSuperMan_BP _ascharacter))
  (Variables|Default|SetSuperMan_BP _asdark_super_man_bp))

(event EventTick
  (params (DeltaSeconds :type Float%20%28single-precision%29))
  (bind _superman_bp (Variables|Default|GetSuperMan_BP))
  (if (> (Math|Vector|VectorLength (Transformation|GetVelocity _superman_bp)) 0.0)
    (Class|MovementComponent|MoveUpdatedComponent (Variables|/Script/Engine.Character|GetCharacterMovement (Variables|Default|GetSuperMan_BP)) "0, 0, 0" (Math|Rotator|MakeRotator 0.0 0.0 (Class|KismetMathLibrary|FixedTurn (Math|Rotator|NormalizeAxis (.yaw (Transformation|GetActorRotation _superman_bp))) (Math|Rotator|NormalizeAxis (.yaw (Pawn|GetControlRotation _superman_bp :!class /Script/Engine.Pawn))) (* DeltaSeconds (Variables|Default|GetRotation%20Yaw%20Rate)))) true)))